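; Dialogue component for the Mouse character, who speaks as a shouting, murderous "VIKING".
; It overrides Dialogue, branching on DialogueTreeIndex and on the option chosen in each AddDialogue step, then clears progress and closes the conversation.
; The second opening reply makes the Viking deal damage to the first-person player and switches the tree index to a shorter repeat rant.
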(fn `dialogue`
  (`parent.dialogue`)
  (switch `int` (`self.dialogueTreeIndex`)
    (:`0`
      (bind (_state _optionindex) (`self.Add Dialogue` "VIKING" "AAAAAAARGGGGG!" (`|MakeArray` "Hi hello there!" "Wha-" :!type "Text")))
      (switch `/Game/dialogueSystem/Enum_Dialogue_State` _state
        (:`NewEnumerator0`
          (switch `int` _optionindex
            (:`0`
              (bind _state_2 (`self.Add Dialogue` "VIKING" "MURDER! KILL! STEAL!" (`|MakeArray` "Continue" :!type "Text")))
              (switch `/Game/dialogueSystem/Enum_Dialogue_State` _state_2
                (:`NewEnumerator0`
                  (`self.clearDialogueProgress`)
                  (`self.closeConvo`))))
            (:`1`
              (bind _state_3 (`self.Add Dialogue` "VIKING" "I KILL YOU!!" (`|MakeArray` "Continue" :!type "Text")))
              (switch `/Game/dialogueSystem/Enum_Dialogue_State` _state_3
                (:`NewEnumerator0`
                  (`self.clearDialogueProgress`)
                  (set `self.dialogueTreeIndex` 1)
                  (`self.closeConvo`)
                  (bind _asbp_first_person_character (cast `/Game/Dynamic/FirstPerson/Blueprints/BP_FirstPersonCharacter` (`GameplayStatics.GetPlayerCharacter` 0)))
                  (`GameplayStatics.ApplyDamage` _asbp_first_person_character 100.0))))))))
    (:`1`
      (bind _state_4 (`self.Add Dialogue` "VIKING" "KILL! KILL! KILL!" (`|MakeArray` "Continue" :!type "Text")))
      (switch `/Game/dialogueSystem/Enum_Dialogue_State` _state_4
        (:`NewEnumerator0`
          (`self.clearDialogueProgress`)
          (`self.closeConvo`))))))