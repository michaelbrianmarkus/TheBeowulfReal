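; Base actor component for branching conversations, which opens and closes a dialogue widget and plays each line's audio and montage.
; The empty Dialogue function, apparently for child overrides, reruns from index -1 whenever the conversation progresses.
; AddDialogue returns the recorded choice for answered steps, otherwise it displays the line, and selecting an option records it and triggers the replay.
; Audio and montages are soft references, async-loaded when not in memory.
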(event `self.ReceiveBeginPlay`
  ;[1 0 0.6929] Load and play audio
  (if (`self.useAudio?`)
    (bind _returnvalue (`|AddComponentByClass` :`self` (`self.GetOwner`) :`Class` "/Script/Engine.AudioComponent"))
    (set `self.audioComp` _returnvalue)))

(event `loadDialogueAudio`
  (params (asset :type "SoundBase Soft Object Reference"))
  ;[1 0 0.6929] Load and play audio
  (bind _object (`|LoadAsset` asset)
    (:`Completed`
      (bind _assound_base (cast `SoundBase` _object))
      (`AudioComponent.SetSound` (`self.audioComp`) _assound_base)
      (`AudioComponent.Play` (`self.audioComp`) 0.0))))

(event `playAnimation`
  (params (MontageToPlay :type "AnimMontage Soft Object Reference") (InSkeletalMeshComponent :type "SkeletalMeshComponent Object Reference"))
  (bind _output (`|ConvertAsset` MontageToPlay))
  ;[1 0 0.6753] loadAndPlayAnimations
  (`/Engine/EditorBlueprintResources/StandardMacros.IsValid` _output
    (:`Is Valid`
      (`self.playLoadedMontage` _output))
    (:`Is Not Valid`
      (bind _object (`|LoadAsset` MontageToPlay)
        (:`Completed`
          (bind _asanim_montage (cast `AnimMontage` _object))
          (`self.playLoadedMontage` _asanim_montage))))))

(event `playLoadedMontage`
  (params (Montage :type "AnimMontage Object Reference"))
  ;[1 0 0.6753] loadAndPlayAnimations
  (`|PlayMontage` (stale `playAnimation` InSkeletalMeshComponent) Montage))

(fn `Add Dialogue`
  (params (Speaker :type Text) (Dialogue :type Text) (Options :type "Array of Text") (dialogueAudio :type "SoundBase Soft Object Reference") (dialogueAnimation :type "AnimMontage Soft Object Reference") (animationTarget :type "SkeletalMeshComponent Object Reference"))
  (returns (State :type "/Game/dialogueSystem/Enum_Dialogue_State Enum") (optionIndex :type Integer))
  (bind (_value _returnvalue) (`BlueprintMapLibrary.Map_Find` (`self.dialogueProgress`) (`self.dialogueIndex`)))
  (`/Engine/EditorBlueprintResources/StandardMacros.IncrementInt` (`self.dialogueIndex`)
    (:`  `
      (if _returnvalue
        (return "NewEnumerator0" _value)
        (else
          (`/Game/Dynamic/UI/HUD_Dialogue.updateDialogueText` (`self.dialogueWidget`) (`self.dialogueIndex`) (`local.Speaker`) (`local.Dialogue`) (`local.Options`))
          (`self.playDialougeAudio` (`local.dialogueAudio`))
          (`self.playAnimation` (`local.dialogueAnimation`) (`local.animationTarget`))
          (return "NewEnumerator1" 0))))))

(fn `clearDialogueProgress`
  (`BlueprintMapLibrary.Map_Clear` (`self.dialogueProgress`)))

(fn `closeConvo`
  (`Widget.RemoveFromParent` (`self.dialogueWidget`))
  (bind _audiocomp (`self.audioComp`)
    (:`then`
      (`AudioComponent.Stop` _audiocomp))
    (:`else`
      _))
  (cast `Character` (`self.GetOwner`))
  (message `/Game/dialogueSystem/BPI_Interactable.convoClosed` (`self.GetOwner`)))

(fn `dialogue`)

(fn `openConvo`
  (bind _returnvalue (`|CreateWidget` "/Game/Dynamic/UI/HUD_Dialogue.HUD_Dialogue_C" null self))
  (bind _output_get (set `self.dialogueWidget` _returnvalue))
  (`UserWidget.AddToViewport` _output_get 0)
  (`self.progressDialogue`))

(fn `playDialougeAudio`
  (params (audio :type "SoundBase Soft Object Reference (by ref)"))
  (bind _output (`|ConvertAsset` (`local.audio`)))
  (if (`KismetSystemLibrary.IsValidSoftObjectReference` audio)
    (`/Engine/EditorBlueprintResources/StandardMacros.IsValid` _output
      (:`Is Valid`
        (`AudioComponent.SetSound` (`self.audioComp`) _output)
        (`AudioComponent.Play` (`self.audioComp`) 0.0))
      (:`Is Not Valid`
        (`self.loadDialogueAudio` (`local.audio`))))))

(fn `progressDialogue`
  (set `self.dialogueIndex` -1)
  (`self.dialogue`))

(fn `removeDialogueProgress`
  (params (progressSteps :type Integer))
  (for _index (range (+ progressSteps 1))
    (`BlueprintMapLibrary.Map_Remove` (`self.dialogueProgress`) (- (`self.dialogueIndex`) _index))))

(fn `setDialogueTreeIndex`
  (params (dialogueTreeIndex :type Integer))
  (set `self.dialogueTreeIndex` dialogueTreeIndex)
  (`self.clearDialogueProgress`))

(fn `updateSelectedOption`
  (params (progressIndex :type "Integer (by ref)") (optionIndex :type "Integer (by ref)"))
  (`BlueprintMapLibrary.Map_Add` (`self.dialogueProgress`) progressIndex optionIndex)
  (`self.progressDialogue`))