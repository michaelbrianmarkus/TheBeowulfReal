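; Base enemy character, apparently a skeleton, that roams, chases and claws the player, then ragdolls and despawns when its health runs out.
; Tick checks planar player distance in two narrow bands, starting a chase at the inner and stopping movement at the outer, otherwise roaming when idle.
; Chase loops through AI MoveTo, briefly enabling an attack collider that damages the player on overlap.
; Roam destinations are random absolute world coordinates, not offsets from the enemy.
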(event `roamAround`
  (bind (_returnvalue_x _returnvalue_y _returnvalue_z) (`KismetMathLibrary.BreakVector` (`SceneComponent.K2_GetComponentLocation` (`self.SkeletalMesh`))))
  (set `CharacterMovementComponent.MaxWalkSpeed` 200.0 (`self.CharacterMovement`))
  (set `self.randomMove?` false)
  (`|AIMoveTo` self (`KismetMathLibrary.MakeVector` (`KismetMathLibrary.RandomFloatInRange` 200.0 400.0) (`KismetMathLibrary.RandomFloatInRange` 200.0 400.0) (+ _returnvalue_z 100.0)) null
    (:`then`
      (`KismetSystemLibrary.Delay` 5.0)
      (set `self.randomMove?` true))))

(event `ChaseBeowulf`
  ;[1 0 0.6634] CHASE THE PLAYER
  (set `CharacterMovementComponent.MaxWalkSpeed` 600.0 (`self.CharacterMovement`))
  (bind _asbp_first_person_character (cast `/Game/Dynamic/FirstPerson/Blueprints/BP_FirstPersonCharacter` (`GameplayStatics.GetPlayerCharacter` 0)))
  (if (not (`/Game/Dynamic/FirstPerson/Blueprints/BP_FirstPersonCharacter.isDead` _asbp_first_person_character))
    (`|AIMoveTo` self (0.0 0.0 0.0) (`GameplayStatics.GetPlayerCharacter` 0) 20.0
      (:`OnSuccess`
        (bind _output_get (set `self.Target` (`KismetMathLibrary.RandomIntegerInRange` 0 1)))
        (set `self.IsAttacking?` true)
        (if (== _output_get 0)
          _
          (else
            _))
        (`KismetSystemLibrary.Delay` 0.5)
        (`GameplayStatics.PlaySoundAtLocation` "/Game/Audio/Skeleton/skeleClaw.skeleClaw" (`SceneComponent.K2_GetComponentLocation` (`self.SkeletalMesh`)) (struct) 0.3 1.0 0.0 null null null null)
        (`PrimitiveComponent.SetCollisionEnabled` (`self.AttackCollision`) "QueryOnly")
        (`KismetSystemLibrary.Delay` 2.0)
        (set `self.IsAttacking?` false)
        (`PrimitiveComponent.SetCollisionEnabled` (`self.AttackCollision`) "NoCollision")
        (`self.ChaseBeowulf`)))))

(event `self.ReceiveTick`
  (params (DeltaSeconds :type "Float (single-precision)"))
  (bind _charactermovement (`self.CharacterMovement`))
  (bind (_returnvalue_x _returnvalue_y) (`KismetMathLibrary.BreakVector` (`SceneComponent.K2_GetComponentLocation` (`self.SkeletalMesh`))))
  (bind _asbp_first_person_character (cast `/Game/Dynamic/FirstPerson/Blueprints/BP_FirstPersonCharacter` (`GameplayStatics.GetPlayerCharacter` 0)))
  (bind (_returnvalue_x_2 _returnvalue_y_2) (`KismetMathLibrary.BreakVector` (`SceneComponent.K2_GetComponentLocation` (`Character.CapsuleComponent` _asbp_first_person_character))))
  (bind _returnvalue (`KismetMathLibrary.Sqrt` (+ (`KismetMathLibrary.Square` (`KismetMathLibrary.Abs` (- _returnvalue_y_2 _returnvalue_y))) (`KismetMathLibrary.Square` (`KismetMathLibrary.Abs` (- _returnvalue_x_2 _returnvalue_x))))))
  (if (and (<= _returnvalue 3522.0) (>= _returnvalue 3422.0))
    (`NavMovementComponent.StopActiveMovement` _charactermovement)
    (elif (and (>= _returnvalue 1326.0) (<= _returnvalue 1426.0))
      (`self.ChaseBeowulf`)
      (elif (== (`MovementComponent.Velocity` _charactermovement) (0.0 0.0 0.0))
        (if (and (not (`self.IsAttacking?`)) (`self.randomMove?`))
          (`self.roamAround`))))))

(event `self.ReceiveBeginPlay`
  (`PrimitiveComponent.SetCollisionEnabled` (`self.AttackCollision`) "NoCollision"))

(event `self.AttackCollision.OnComponentBeginOverlap`
  (params (OverlappedComponent :type "PrimitiveComponent Object Reference") (OtherActor :type "Actor Object Reference") (OtherComp :type "PrimitiveComponent Object Reference") (OtherBodyIndex :type Integer) (bFromSweep :type Boolean) (SweepResult :type "HitResult Structure (by ref)"))
  ;[1 0 0.5828] AttackHitPlayer
  (bind _asbp_first_person_character (cast `/Game/Dynamic/FirstPerson/Blueprints/BP_FirstPersonCharacter` OtherActor))
  (bind _asbp_first_person_character_2 (cast `/Game/Dynamic/FirstPerson/Blueprints/BP_FirstPersonCharacter` (`GameplayStatics.GetPlayerCharacter` 0)))
  (if (not (`/Game/Dynamic/FirstPerson/Blueprints/BP_FirstPersonCharacter.isDead` _asbp_first_person_character_2))
    (`GameplayStatics.ApplyDamage` _asbp_first_person_character 3.0)))

(event `self.ReceiveAnyDamage`
  (params (Damage :type "Float (single-precision)") (DamageType :type "DamageType Object Reference") (InstigatedBy :type "Controller Object Reference") (DamageCauser :type "Actor Object Reference"))
  ;[1 0 0.5763] Death
  (bind _output_get (set `self.Health` (- (`self.Health`) Damage)))
  (if (<= _output_get 0.0)
    (`PrimitiveComponent.SetSimulatePhysics` (`self.SkeletalMesh`) true)
    (`CharacterMovementComponent.DisableMovement` (`self.CharacterMovement`))
    (`PrimitiveComponent.SetCollisionEnabled` (`self.AttackCollision`) "NoCollision")
    (`KismetSystemLibrary.Delay` 5.0)
    (`self.K2_DestroyActor`)))

(event `self.characterCollision.OnComponentBeginOverlap`
  (params (OverlappedComponent :type "PrimitiveComponent Object Reference") (OtherActor :type "Actor Object Reference") (OtherComp :type "PrimitiveComponent Object Reference") (OtherBodyIndex :type Integer) (bFromSweep :type Boolean) (SweepResult :type "HitResult Structure (by ref)")))

(fn `staminaDrain`)

(fn `UserConstructionScript`)