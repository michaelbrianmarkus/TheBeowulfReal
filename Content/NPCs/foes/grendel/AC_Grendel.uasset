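; Grendel's dialogue component, which runs the branching conversation that leads to a fight or a peaceful exit.
; Dialogue overrides its parent with nested AddDialogue choices, including a reconciliation branch that loops to the greeting and a leave option that loads Herot2.
; Attack choices turn Grendel hostile, enable physics on tables and explosive barrels, start his charge-attack check and show his widget.
; Grendel is found by casting the first NPC_Base in the level.
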(fn `dialogue`
  (`parent.dialogue`)
  (bind _returnvalue (`GameplayStatics.GetActorOfClass` "/Game/dialogueSystem/NPC_Base.NPC_Base_C"))
  (bind _asnpc_grendel (cast `/Game/NPCs/foes/grendel/NPC_Grendel` _returnvalue))
  (switch `int` (`self.dialogueTreeIndex`)
    (:`0`
      (bind _state (`self.Add Dialogue` "The Foul Beast" "Oh hey! A new friend! Welcome into my house, It's great to meet you!" (`|MakeArray` "Continue" :!type "Text") null "/Game/NPCs/friends/THEKING/HrothgarTalking_InFront.HrothgarTalking_InFront" :!label _label))
      (switch `/Game/dialogueSystem/Enum_Dialogue_State` _state
        (:`NewEnumerator0`
          (bind (_state_2 _optionindex) (`self.Add Dialogue` "Grendel" "The name's Grendel, what's yours?" (`|MakeArray` "You won't trick me with your deception, you sick monster!" "The names Beowulf, thank you kindly for the warm greeting." "The man who's name will be the last thing you mutter... (Attack)" :!type "Text") null "/Game/NPCs/friends/THEKING/HrothgarTalking_InFront.HrothgarTalking_InFront"))
          (switch `/Game/dialogueSystem/Enum_Dialogue_State` _state_2
            (:`NewEnumerator0`
              (switch `int` _optionindex
                (:`0`
                  (bind _state_3 (`self.Add Dialogue` "Grendel" "Why, that's proposperous! I am just as intelligent a creature as you humans are! Why do you kingdom types allways treat me like this!" (`|MakeArray` "Continue" :!type "Text") null "/Game/NPCs/friends/THEKING/HrothgarTalking_InFront.HrothgarTalking_InFront"))
                  (switch `/Game/dialogueSystem/Enum_Dialogue_State` _state_3
                    (:`NewEnumerator0`
                      (bind _state_4 (`self.Add Dialogue` "Grendel" "...." (`|MakeArray` "Continue" :!type "Text") null "/Game/NPCs/friends/THEKING/HrothgarTalking_InFront.HrothgarTalking_InFront"))
                      (switch `/Game/dialogueSystem/Enum_Dialogue_State` _state_4
                        (:`NewEnumerator0`
                          (bind _state_5 (`self.Add Dialogue` "Grendel" "Look, I'm terribly sorry for ranting on, what a bad first impression! Can we start over and make amends?" (`|MakeArray` "Continue" :!type "Text") null "/Game/NPCs/friends/THEKING/HrothgarTalking_InFront.HrothgarTalking_InFront"))
                          (switch `/Game/dialogueSystem/Enum_Dialogue_State` _state_5
                            (:`NewEnumerator0`
                              (bind (_state_6 _optionindex_2) (`self.Add Dialogue` "Grendel" "...." (`|MakeArray` "Alright, I'll give you another shot." "The only amends I make, are in BLOOD! (Attack)" :!type "Text") null "/Game/NPCs/friends/THEKING/HrothgarTalking_InFront.HrothgarTalking_InFront"))
                              (switch `/Game/dialogueSystem/Enum_Dialogue_State` _state_6
                                (:`NewEnumerator0`
                                  (switch `int` _optionindex_2
                                    (:`0`
                                      (goto _label))
                                    (:`1`
                                      (`self.closeConvo` :!label _label_2)
                                      (set `/Game/NPCs/foes/grendel/NPC_Grendel.hostile?` true _asnpc_grendel)
                                      (bind _outactors (`GameplayStatics.GetAllActorsOfClass` "/Game/Props/GrendelHome/tables.tables_C"))
                                      (for _array_element _outactors
                                        (`/Game/Props/GrendelHome/tables.simulatePhys` _array_element))
                                      (bind _outactors_2 (`GameplayStatics.GetAllActorsOfClass` "/Game/Props/GrendelHome/explosiveBarrels.explosiveBarrels_C"))
                                      (for _array_element_2 _outactors_2
                                        (`PrimitiveComponent.SetSimulatePhysics` (`/Game/Props/GrendelHome/explosiveBarrels.StaticMesh` _array_element_2) true))
                                      (`/Game/NPCs/foes/grendel/NPC_Grendel.HostileState` _asnpc_grendel)
                                      (`/Game/NPCs/foes/grendel/NPC_Grendel.chargeAttackChecker` _asnpc_grendel)
                                      (`SceneComponent.SetVisibility` (`/Game/NPCs/foes/grendel/NPC_Grendel.Widget` _asnpc_grendel) true false))))))))))))
                (:`1`
                  (bind (_state_7 _optionindex_3) (`self.Add Dialogue` "Grendel" "You're welcome! Anyways, what did you want from me?" (`|MakeArray` "I kind of have to kill you.... sorry? (Attack)" "I was just leaving actually" :!type "Text") null "/Game/NPCs/friends/THEKING/HrothgarTalking_InFront.HrothgarTalking_InFront"))
                  (switch `/Game/dialogueSystem/Enum_Dialogue_State` _state_7
                    (:`NewEnumerator0`
                      (switch `int` _optionindex_3
                        (:`0`
                          (goto _label_2))
                        (:`1`
                          (`GameplayStatics.OpenLevelBySoftObjectPtr` "/Game/Dynamic/FirstPerson/Maps/Herot2.Herot2"))))))
                (:`2`
                  (goto _label_2))))))))))