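; Dialogue component for the Bandit King NPC, who guards a bridge crossing at a bandit camp.
; Overrides Dialogue with a single tree (index 0) of nested AddDialogue calls, branching on chosen options and carrying voice audio and animation.
; A Fame check on the player decides between free passage and a refusal that can lead to a gnome-spying favor.
; Outcomes, including the hostile option, are only spoken; no quest or hostility state is set here.
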(fn `dialogue`
  (`parent.dialogue`)
  (bind _asbp_first_person_character (cast `/Game/Dynamic/FirstPerson/Blueprints/BP_FirstPersonCharacter` (`GameplayStatics.GetPlayerCharacter` 0)))
  (`GameplayStatics.GetActorOfClass` "/Game/NPCs/friends/BanditKing/NPC_BanditKing.NPC_BanditKing_C")
  (switch `int` (`self.dialogueTreeIndex`)
    (:`0`
      (bind _state (`self.Add Dialogue` "Bandit King" "You know where you are, fresh meat?" (`|MakeArray` "Continue" :!type "Text") "/Game/Audio/VoiceLines/banditKing/banditKing-01.banditKing-01" "/Game/NPCs/friends/THEKING/HrothgarTalking_InFront.HrothgarTalking_InFront"))
      (switch `/Game/dialogueSystem/Enum_Dialogue_State` _state
        (:`NewEnumerator0`
          (bind _state_2 (`self.Add Dialogue` "Bandit King" "Since you haven’t figured it out yet, lemme clue you in. This is the pack’s den. The meanest and toughest of all bandit camps." (`|MakeArray` "Continue" :!type "Text") "/Game/Audio/VoiceLines/banditKing/banditKing-02.banditKing-02" "/Game/NPCs/friends/THEKING/HrothgarTalking_InFront.HrothgarTalking_InFront"))
          (switch `/Game/dialogueSystem/Enum_Dialogue_State` _state_2
            (:`NewEnumerator0`
              (bind (_state_3 _optionindex) (`self.Add Dialogue` "Bandit King" "But don’t worry, fresh meat, we don’t bite… so long as you play by our rules that is." (`|MakeArray` "I need to get across that bridge" " I’m getting across that bridge no matter  \nwhat you say. (Hostile Camp)" :!type "Text") "/Game/Audio/VoiceLines/banditKing/banditKing-03.banditKing-03" "/Game/NPCs/friends/THEKING/HrothgarTalking_InFront.HrothgarTalking_InFront"))
              (switch `/Game/dialogueSystem/Enum_Dialogue_State` _state_3
                (:`NewEnumerator0`
                  (switch `int` _optionindex
                    (:`0`
                      (if (>= (`/Game/Dynamic/FirstPerson/Blueprints/BP_FirstPersonCharacter.Fame` _asbp_first_person_character) 50.0)
                        (bind _state_4 (`self.Add Dialogue` "Bandit King" "Wait a minute… It's YOU." (`|MakeArray` "Continue" :!type "Text") "/Game/Audio/VoiceLines/banditKing/banditKing-04.banditKing-04" "/Game/NPCs/friends/THEKING/HrothgarTalking_InFront.HrothgarTalking_InFront"))
                        (switch `/Game/dialogueSystem/Enum_Dialogue_State` _state_4
                          (:`NewEnumerator0`
                            (bind _state_5 (`self.Add Dialogue` "Bandit King" "You’re that guy who's been going around makin a name fer yerself." (`|MakeArray` "Continue" :!type "Text") "/Game/Audio/VoiceLines/banditKing/banditKing-05.banditKing-05" "/Game/NPCs/friends/THEKING/HrothgarTalking_InFront.HrothgarTalking_InFront"))
                            (switch `/Game/dialogueSystem/Enum_Dialogue_State` _state_5
                              (:`NewEnumerator0`
                                (bind _state_6 (`self.Add Dialogue` "Bandit King" "HAHAHA!" (`|MakeArray` "Continue" :!type "Text") "/Game/Audio/VoiceLines/banditKing/banditKing-06.banditKing-06" "/Game/NPCs/friends/THEKING/HrothgarTalking_InFront.HrothgarTalking_InFront"))
                                (switch `/Game/dialogueSystem/Enum_Dialogue_State` _state_6
                                  (:`NewEnumerator0`
                                    (bind _state_7 (`self.Add Dialogue` "Bandit King" "I like your attitude! Y’know what you can cross, free of charge. " (`|MakeArray` "Continue" :!type "Text") "/Game/Audio/VoiceLines/banditKing/banditKing-07.banditKing-07" "/Game/NPCs/friends/THEKING/HrothgarTalking_InFront.HrothgarTalking_InFront"))
                                    (switch `/Game/dialogueSystem/Enum_Dialogue_State` _state_7)))))))
                        (else
                          (bind _state_8 (`self.Add Dialogue` "Bandit King" "HEH! FAT CHANCE LOSER!" (`|MakeArray` "Continue" :!type "Text") "/Game/Audio/VoiceLines/banditKing/banditKing-08.banditKing-08" "/Game/NPCs/friends/THEKING/HrothgarTalking_InFront.HrothgarTalking_InFront"))
                          (switch `/Game/dialogueSystem/Enum_Dialogue_State` _state_8
                            (:`NewEnumerator0`
                              (bind _state_9 (`self.Add Dialogue` "Bandit King" "We don’t just let anyone cross this bridge! " (`|MakeArray` "Continue" :!type "Text") "/Game/Audio/VoiceLines/banditKing/banditKing-09.banditKing-09" "/Game/NPCs/friends/THEKING/HrothgarTalking_InFront.HrothgarTalking_InFront"))
                              (switch `/Game/dialogueSystem/Enum_Dialogue_State` _state_9
                                (:`NewEnumerator0`
                                  (bind (_state_10 _optionindex_2) (`self.Add Dialogue` "Bandit King" "Don’t care if you from that fancy kingdom either! Round here, your laws mean nothing man. " (`|MakeArray` "Aw c’mon man, isn’t there anything I can do?" "I’ll be back later" :!type "Text") "/Game/Audio/VoiceLines/banditKing/banditKing-10.banditKing-10" "/Game/NPCs/friends/THEKING/HrothgarTalking_InFront.HrothgarTalking_InFront"))
                                  (switch `/Game/dialogueSystem/Enum_Dialogue_State` _state_10
                                    (:`NewEnumerator0`
                                      (switch `int` _optionindex_2
                                        (:`0`
                                          (bind _state_11 (`self.Add Dialogue` "Bandit King" "Hmmm. You look like the morally questionable type. And you’re an unknown face too…If you really want to cross that bridge I’m going to need a favor in return, holmes." (`|MakeArray` "Continue" :!type "Text") "/Game/Audio/VoiceLines/banditKing/banditKing-11.banditKing-11" "/Game/NPCs/friends/THEKING/HrothgarTalking_InFront.HrothgarTalking_InFront"))
                                          (switch `/Game/dialogueSystem/Enum_Dialogue_State` _state_11
                                            (:`NewEnumerator0`
                                              (bind _state_12 (`self.Add Dialogue` "Beowulf" "And that is?" (`|MakeArray` "Continue" :!type "Text") null "/Game/NPCs/friends/THEKING/HrothgarTalking_InFront.HrothgarTalking_InFront"))
                                              (switch `/Game/dialogueSystem/Enum_Dialogue_State` _state_12
                                                (:`NewEnumerator0`
                                                  (bind _state_13 (`self.Add Dialogue` "Bandit King" "I want you to figure out whatever the hell the gnomes are up to, man!" (`|MakeArray` "Continue" :!type "Text") "/Game/Audio/VoiceLines/banditKing/banditKing-12.banditKing-12" "/Game/NPCs/friends/THEKING/HrothgarTalking_InFront.HrothgarTalking_InFront"))
                                                  (switch `/Game/dialogueSystem/Enum_Dialogue_State` _state_13
                                                    (:`NewEnumerator0`
                                                      (bind _state_14 (`self.Add Dialogue` "Beowulf" "Forreal?!" (`|MakeArray` "Continue" :!type "Text") null "/Game/NPCs/friends/THEKING/HrothgarTalking_InFront.HrothgarTalking_InFront"))
                                                      (switch `/Game/dialogueSystem/Enum_Dialogue_State` _state_14
                                                        (:`NewEnumerator0`
                                                          (bind _state_15 (`self.Add Dialogue` "Bandit King" "Believe it or not ese, but the gnomes are the bandit’s sworn enemy. We been fighting gang wars since back in the starving times." (`|MakeArray` "Continue" :!type "Text") "/Game/Audio/VoiceLines/banditKing/banditKing-13.banditKing-13" "/Game/NPCs/friends/THEKING/HrothgarTalking_InFront.HrothgarTalking_InFront"))
                                                          (switch `/Game/dialogueSystem/Enum_Dialogue_State` _state_15
                                                            (:`NewEnumerator0`
                                                              (bind _state_16 (`self.Add Dialogue` "Bandit King" "Those little pendejos are always scheming something, and I have my suspicions that they are responsible for the resurgence of the pixie dust!" (`|MakeArray` "Continue" :!type "Text") "/Game/Audio/VoiceLines/banditKing/banditKing-14.banditKing-14" "/Game/NPCs/friends/THEKING/HrothgarTalking_InFront.HrothgarTalking_InFront"))
                                                              (switch `/Game/dialogueSystem/Enum_Dialogue_State` _state_16
                                                                (:`NewEnumerator0`
                                                                  (bind _state_17 (`self.Add Dialogue` "Bandit King" " I can’t say for sure tho, and storming their grandfather tree with my gang is an invitation for war. That’s where you come in holmes." (`|MakeArray` "Continue" :!type "Text") "/Game/Audio/VoiceLines/banditKing/banditKing-15.banditKing-15" "/Game/NPCs/friends/THEKING/HrothgarTalking_InFront.HrothgarTalking_InFront"))
                                                                  (switch `/Game/dialogueSystem/Enum_Dialogue_State` _state_17
                                                                    (:`NewEnumerator0`
                                                                      (bind _state_18 (`self.Add Dialogue` "Bandit King" " You be my eyes and ears and get me proof of whatever the hell they’re up to in there, okay?" (`|MakeArray` "Continue" :!type "Text") "/Game/Audio/VoiceLines/banditKing/banditKing-16.banditKing-16" "/Game/NPCs/friends/THEKING/HrothgarTalking_InFront.HrothgarTalking_InFront"))
                                                                      (switch `/Game/dialogueSystem/Enum_Dialogue_State` _state_18
                                                                        (:`NewEnumerator0`
                                                                          (bind _state_19 (`self.Add Dialogue` "Beowulf" "Sure thing, holmes." (`|MakeArray` "Continue" :!type "Text") null "/Game/NPCs/friends/THEKING/HrothgarTalking_InFront.HrothgarTalking_InFront"))
                                                                          (switch `/Game/dialogueSystem/Enum_Dialogue_State` _state_19))))))))))))))))))
                                        (:`1`
                                          (bind _state_20 (`self.Add Dialogue` "Bandit King" "Sure, whatever ese." (`|MakeArray` "Aw c’mon man, isn’t there anything I can do?" "I’ll be back later" :!type "Text") "/Game/Audio/VoiceLines/banditKing/banditKing-17.banditKing-17" "/Game/NPCs/friends/THEKING/HrothgarTalking_InFront.HrothgarTalking_InFront"))
                                          (switch `/Game/dialogueSystem/Enum_Dialogue_State` _state_20))))))))))))
                    (:`1`
                      (bind _state_21 (`self.Add Dialogue` "Bandit King" "HEH! FAT CHANCE LOSER!" (`|MakeArray` "Continue" :!type "Text") "/Game/Audio/VoiceLines/banditKing/banditKing-08.banditKing-08" "/Game/NPCs/friends/THEKING/HrothgarTalking_InFront.HrothgarTalking_InFront"))
                      (switch `/Game/dialogueSystem/Enum_Dialogue_State` _state_21))))))))))))