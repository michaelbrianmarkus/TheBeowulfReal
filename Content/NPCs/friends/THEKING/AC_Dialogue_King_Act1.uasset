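; Dialogue component for King Hrothgar's Act 1 throne-room scene, where Beowulf is offered the quest to kill Grendel and Sir Aeschere objects.
; It picks a branch from the saved KingDialogueTreeIndex and chains AddDialogue nodes with speaker, text, voice audio and animations targeting the king or knight mesh.
; Refusing makes the knight kill Beowulf, while accepting sends the knight off and opens a looping question menu with the king.
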(fn `dialogue`
  (set `self.kingAnimationSkeleton` (`Actor.GetComponentByClass` (`self.GetOwner`) "/Script/Engine.SkeletalMeshComponent"))
  (`parent.dialogue`)
  (bind _returnvalue (`GameplayStatics.GetActorOfClass` "/Game/dialogueSystem/NPC_Base.NPC_Base_C"))
  (bind _asnpc_knight (cast `/Game/NPCs/friends/Knight/NPC_Knight` _returnvalue))
  (bind _asbp_first_person_character (cast `/Game/Dynamic/FirstPerson/Blueprints/BP_FirstPersonCharacter` (`GameplayStatics.GetPlayerCharacter` 0)))
  (bind _as_level_save_data (`/Game/Dynamic/FirstPerson/Blueprints/BP_FirstPersonGameMode.As Level Save Data` (`/Game/Dynamic/FirstPerson/Blueprints/BP_FirstPersonCharacter.Game Mode` _asbp_first_person_character)))
  (set `self.dialogueTreeIndex` (`/Game/Dynamic/FirstPerson/Blueprints/levelSaveData.kingDialogueTreeIndex` _as_level_save_data))
  (set `self.knightAnimationSkeleton` (`Character.Mesh` _asnpc_knight))
  (switch `int` (`self.dialogueTreeIndex`)
    (:`0`
      (bind _state (`self.Add Dialogue` "Beowulf" "*Yawn*  Yeah, that was a splendid nap. Oh what's going on here..." (`|MakeArray` "Continue" :!type "Text") null "/Game/NPCs/friends/THEKING/HrothgarTalking_InFront.HrothgarTalking_InFront" (`self.kingAnimationSkeleton`)))
      (switch `/Game/dialogueSystem/Enum_Dialogue_State` _state
        (:`NewEnumerator0`
          (bind _state_2 (`self.Add Dialogue` "King Hrothgar" "What does thy mean thine forces is not great enough to defeat one measly goblin!" (`|MakeArray` "Continue" :!type "Text") "/Game/Audio/VoiceLines/KingHrothgar/king-01.king-01" "/Game/NPCs/friends/THEKING/HrothgarDisbeliefHeadDownn.HrothgarDisbeliefHeadDownn" (`self.kingAnimationSkeleton`)))
          (switch `/Game/dialogueSystem/Enum_Dialogue_State` _state_2
            (:`NewEnumerator0`
              (bind _state_3 (`self.Add Dialogue` "Sir Aeschere" "My lord, every platoon we sent out has yet to return. This foul beast hath massacared many of mine best knights." (`|MakeArray` "Continue" :!type "Text") null "/Game/NPCs/friends/Knight/knight_talk_To_King.knight_talk_To_King" (`self.knightAnimationSkeleton`)))
              (switch `/Game/dialogueSystem/Enum_Dialogue_State` _state_3
                (:`NewEnumerator0`
                  (bind _state_4 (`self.Add Dialogue` "Sir Aeschere" "The kingdom's subjects are taking note of the bloodshed, and are beginning to lose faith in you my liege.  Thine goblin has become a matter of uptmost importance. " (`|MakeArray` "Continue" :!type "Text") null "/Game/NPCs/friends/Knight/knight_look_To_King.knight_look_To_King" (`self.knightAnimationSkeleton`)))
                  (switch `/Game/dialogueSystem/Enum_Dialogue_State` _state_4
                    (:`NewEnumerator0`
                      (bind _state_5 (`self.Add Dialogue` "King Hrothgar" "So what does thine, suppose I do? " (`|MakeArray` "Continue" :!type "Text") "/Game/Audio/VoiceLines/KingHrothgar/king-02.king-02" "/Game/NPCs/friends/THEKING/HrothgarTalking_InFront.HrothgarTalking_InFront" (`self.kingAnimationSkeleton`)))
                      (switch `/Game/dialogueSystem/Enum_Dialogue_State` _state_5
                        (:`NewEnumerator0`
                          (bind _state_6 (`self.Add Dialogue` "Sir Aeschere" "My lord, I propose we lay an ambush for the beast by luring it near our castle walls and then- " (`|MakeArray` "Continue" :!type "Text") null "/Game/NPCs/friends/Knight/knight_talk_To_King.knight_talk_To_King" (`self.knightAnimationSkeleton`)))
                          (switch `/Game/dialogueSystem/Enum_Dialogue_State` _state_6
                            (:`NewEnumerator0`
                              (bind _state_7 (`self.Add Dialogue` "Sir Aeschere" "What the!" (`|MakeArray` "Continue" :!type "Text") null "/Game/NPCs/friends/Knight/knight_Notice_beowulf.knight_Notice_beowulf" (`self.knightAnimationSkeleton`)))
                              (switch `/Game/dialogueSystem/Enum_Dialogue_State` _state_7
                                (:`NewEnumerator0`
                                  (bind _state_8 (`self.Add Dialogue` "King Hrothgar" "Forsooth, I say! Spit it out Aeschere! " (`|MakeArray` "Continue" :!type "Text") "/Game/Audio/VoiceLines/KingHrothgar/king-03.king-03"))
                                  (switch `/Game/dialogueSystem/Enum_Dialogue_State` _state_8
                                    (:`NewEnumerator0`
                                      (bind _state_9 (`self.Add Dialogue` "Sir Aeschere" "Forgive my inquiry my lord, but wherefore is thither a peasant living in thine royal throneroom? " (`|MakeArray` "Continue" :!type "Text") null "/Game/NPCs/friends/Knight/knight_Notice_lookKing.knight_Notice_lookKing" (`self.knightAnimationSkeleton`)))
                                      (switch `/Game/dialogueSystem/Enum_Dialogue_State` _state_9
                                        (:`NewEnumerator0`
                                          (bind _state_10 (`self.Add Dialogue` "King Hrothgar" "What is thou mumbling about- Oh." (`|MakeArray` "Continue" :!type "Text") "/Game/Audio/VoiceLines/KingHrothgar/king-04.king-04" "/Game/NPCs/friends/THEKING/Hrothgar_LookAtBeowulf.Hrothgar_LookAtBeowulf" (`self.kingAnimationSkeleton`)))
                                          (switch `/Game/dialogueSystem/Enum_Dialogue_State` _state_10
                                            (:`NewEnumerator0`
                                              (bind _state_11 (`self.Add Dialogue` "King Hrothgar" "What the devils! Who let this riffraff inside my royal castle!" (`|MakeArray` "Continue" :!type "Text") "/Game/Audio/VoiceLines/KingHrothgar/king-05.king-05" "/Game/NPCs/friends/Knight/knight_Notice_beowulf.knight_Notice_beowulf" (`self.knightAnimationSkeleton`)))
                                              (switch `/Game/dialogueSystem/Enum_Dialogue_State` _state_11
                                                (:`NewEnumerator0`
                                                  (bind _state_12 (`self.Add Dialogue` "Sir Aeschere" "Wish for me to dispose of this one, my king?" (`|MakeArray` "Continue" :!type "Text") null "/Game/NPCs/friends/Knight/knight_Notice_lookKing.knight_Notice_lookKing" (`self.knightAnimationSkeleton`)))
                                                  (switch `/Game/dialogueSystem/Enum_Dialogue_State` _state_12
                                                    (:`NewEnumerator0`
                                                      (bind _state_13 (`self.Add Dialogue` "King Hrothgar" "Stand down, Aeschere! Hmmm. What an interesting one..." (`|MakeArray` "Continue" :!type "Text") "/Game/Audio/VoiceLines/KingHrothgar/king-06.king-06" "/Game/NPCs/friends/Knight/knight_Notice_beowulf.knight_Notice_beowulf" (`self.knightAnimationSkeleton`)))
                                                      (switch `/Game/dialogueSystem/Enum_Dialogue_State` _state_13
                                                        (:`NewEnumerator0`
                                                          (bind _state_14 (`self.Add Dialogue` "King Hrothgar" "You there! You seem like you have quite the build, hath you experience with the blade?" (`|MakeArray` "Continue" :!type "Text") "/Game/Audio/VoiceLines/KingHrothgar/king-07.king-07"))
                                                          (switch `/Game/dialogueSystem/Enum_Dialogue_State` _state_14
                                                            (:`NewEnumerator0`
                                                              (bind _state_15 (`self.Add Dialogue` "Beowulf" "Yep." (`|MakeArray` "Continue" :!type "Text")))
                                                              (switch `/Game/dialogueSystem/Enum_Dialogue_State` _state_15
                                                                (:`NewEnumerator0`
                                                                  (bind _state_16 (`self.Add Dialogue` "King Hrothgar" "Then I shall make you a knight of my kingdom! It is with great honor for you to obey the royal decree of......" (`|MakeArray` "Continue" :!type "Text") "/Game/Audio/VoiceLines/KingHrothgar/king-08.king-08"))
                                                                  (switch `/Game/dialogueSystem/Enum_Dialogue_State` _state_16
                                                                    (:`NewEnumerator0`
                                                                      (bind _state_17 (`self.Add Dialogue` "King Hrothgar" "Killing the ugly troll living in a shack across the road." (`|MakeArray` "Continue" :!type "Text") "/Game/Audio/VoiceLines/KingHrothgar/king-09.king-09"))
                                                                      (switch `/Game/dialogueSystem/Enum_Dialogue_State` _state_17
                                                                        (:`NewEnumerator0`
                                                                          (bind _state_18 (`self.Add Dialogue` "Beowulf" "Sure, I don't see why not." (`|MakeArray` "Continue" :!type "Text")))
                                                                          (switch `/Game/dialogueSystem/Enum_Dialogue_State` _state_18
                                                                            (:`NewEnumerator0`
                                                                              (bind _state_19 (`self.Add Dialogue` "Sir Aeschere" "Wha? Wh-Why??? Who?!??" (`|MakeArray` "Continue" :!type "Text") null "/Game/NPCs/friends/Knight/knight_Disbelief.knight_Disbelief" (`self.knightAnimationSkeleton`)))
                                                                              (switch `/Game/dialogueSystem/Enum_Dialogue_State` _state_19
                                                                                (:`NewEnumerator0`
                                                                                  (bind _state_20 (`self.Add Dialogue` "King Hrothgar" "Is something the matter, Aeschere?" (`|MakeArray` "Continue" :!type "Text") "/Game/Audio/VoiceLines/KingHrothgar/king-10.king-10" "/Game/NPCs/friends/THEKING/HrothgarTalking_InFront.HrothgarTalking_InFront" (`self.kingAnimationSkeleton`)))
                                                                                  (switch `/Game/dialogueSystem/Enum_Dialogue_State` _state_20
                                                                                    (:`NewEnumerator0`
                                                                                      (bind _state_21 (`self.Add Dialogue` "Sir Aeschere" "My lord, in my 21 years on this Earth serving under your command, I have not once questioned your leadership, but....this, is er- unprecedented. May I implore why him?" (`|MakeArray` "Continue" :!type "Text") null "/Game/NPCs/friends/Knight/knight_look_To_King.knight_look_To_King" (`self.knightAnimationSkeleton`)))
                                                                                      (switch `/Game/dialogueSystem/Enum_Dialogue_State` _state_21
                                                                                        (:`NewEnumerator0`
                                                                                          (bind _state_22 (`self.Add Dialogue` "King Hrothgar" "This peasant had the bravery to sleep in my throneroom with so much skill that not even my best knight could've detected him momentarily. I adore his moxie." (`|MakeArray` "Continue" :!type "Text") "/Game/Audio/VoiceLines/KingHrothgar/king-11.king-11" "/Game/NPCs/friends/THEKING/Hrothgar_LookAtBeowulf.Hrothgar_LookAtBeowulf" (`self.kingAnimationSkeleton`)))
                                                                                          (switch `/Game/dialogueSystem/Enum_Dialogue_State` _state_22
                                                                                            (:`NewEnumerator0`
                                                                                              (bind _state_23 (`self.Add Dialogue` "Sir Aeschere" "This is tomfoolery to the upmost extent! Thine doesn't even know if thy is skillful enough for such a beast! " (`|MakeArray` "Continue" :!type "Text") null "/Game/NPCs/friends/Knight/knight_Disbelief.knight_Disbelief" (`self.knightAnimationSkeleton`)))
                                                                                              (switch `/Game/dialogueSystem/Enum_Dialogue_State` _state_23
                                                                                                (:`NewEnumerator0`
                                                                                                  (bind _state_24 (`self.Add Dialogue` "King Hrothgar" "Settle down, Aeschere! Forsooth, he said he is experienced with the blade himself, for he must be a natural! For this fact alone, I trust him with mine life." (`|MakeArray` "Continue" :!type "Text") "/Game/Audio/VoiceLines/KingHrothgar/king-12.king-12" "/Game/NPCs/friends/THEKING/HrothgarTalking_InFront.HrothgarTalking_InFront" (`self.kingAnimationSkeleton`)))
                                                                                                  (switch `/Game/dialogueSystem/Enum_Dialogue_State` _state_24
                                                                                                    (:`NewEnumerator0`
                                                                                                      (bind _state_25 (`self.Add Dialogue` "Sir Aeschere" "My lord..." (`|MakeArray` "Continue" :!type "Text") null "/Game/NPCs/friends/Knight/knight_Notice_beowulf.knight_Notice_beowulf" (`self.knightAnimationSkeleton`)))
                                                                                                      (switch `/Game/dialogueSystem/Enum_Dialogue_State` _state_25
                                                                                                        (:`NewEnumerator0`
                                                                                                          (bind (_state_26 _optionindex) (`self.Add Dialogue` "King Hrothgar" "What do you say peasant? Will you take the quest to strike down this foul, grotesque, smelly,  ugly, heinous, and downright despicable beast that has been terrorizing our kingdom for millennia?" (`|MakeArray` "I changed my mind." "GIVE ME BLOOD!" :!type "Text") "/Game/Audio/VoiceLines/KingHrothgar/king-13.king-13" "/Game/NPCs/friends/THEKING/Hrothgar_LookAtBeowulf.Hrothgar_LookAtBeowulf" (`self.kingAnimationSkeleton`)))
                                                                                                          (switch `/Game/dialogueSystem/Enum_Dialogue_State` _state_26
                                                                                                            (:`NewEnumerator0`
                                                                                                              (switch `int` _optionindex
                                                                                                                (:`0`
                                                                                                                  (bind _state_27 (`self.Add Dialogue` "King Hrothgar" "Y'know what, I changed MY mind. Aeschere, kill him." (`|MakeArray` "Continue" :!type "Text") "/Game/Audio/VoiceLines/KingHrothgar/king-14.king-14" "/Game/NPCs/friends/THEKING/HrothgarTalking_InFront.HrothgarTalking_InFront" (`self.kingAnimationSkeleton`)))
                                                                                                                  (switch `/Game/dialogueSystem/Enum_Dialogue_State` _state_27
                                                                                                                    (:`NewEnumerator0`
                                                                                                                      (bind _state_28 (`self.Add Dialogue` "Sir Aeschere" "At your command, my liege." (`|MakeArray` "Continue" :!type "Text") null "/Game/NPCs/friends/THEKING/Hrothgar_LookAtBeowulf.Hrothgar_LookAtBeowulf" (`self.kingAnimationSkeleton`)))
                                                                                                                      (switch `/Game/dialogueSystem/Enum_Dialogue_State` _state_28
                                                                                                                        (:`NewEnumerator0`
                                                                                                                          (`self.clearDialogueProgress`)
                                                                                                                          (`self.closeConvo`)
                                                                                                                          (`/Game/NPCs/friends/Knight/NPC_Knight.killBeowulf` _asnpc_knight))))))
                                                                                                                (:`1`
                                                                                                                  (bind _state_29 (`self.Add Dialogue` "King Hrothgar" "See Aeschere? This man is more than capable of battling that foul beast! If you're still not convinced then how bout' you test his ability in the training grounds? Eh Aeschere?" (`|MakeArray` "Continue" :!type "Text") "/Game/Audio/VoiceLines/KingHrothgar/king-15.king-15" "/Game/NPCs/friends/THEKING/HrothgarTalking_InFront.HrothgarTalking_InFront" (`self.kingAnimationSkeleton`)))
                                                                                                                  (switch `/Game/dialogueSystem/Enum_Dialogue_State` _state_29
                                                                                                                    (:`NewEnumerator0`
                                                                                                                      (bind _state_30 (`self.Add Dialogue` "Sir Aeschere" "I-Uh, suppose it wouldn't be fatal to inquire his combative ability." (`|MakeArray` "Continue" :!type "Text") null "/Game/NPCs/friends/Knight/knight_Notice_lookKing.knight_Notice_lookKing" (`self.knightAnimationSkeleton`)))
                                                                                                                      (switch `/Game/dialogueSystem/Enum_Dialogue_State` _state_30
                                                                                                                        (:`NewEnumerator0`
                                                                                                                          (bind _state_31 (`self.Add Dialogue` "Sir Aeschere" "Peasant,  if you wish to test your ability, meet me in the training grounds to the left when you exit the royal castle, I'll be waiting." (`|MakeArray` "Continue" :!type "Text") null "/Game/NPCs/friends/Knight/knight_Notice_beowulf.knight_Notice_beowulf" (`self.knightAnimationSkeleton`)))
                                                                                                                          (switch `/Game/dialogueSystem/Enum_Dialogue_State` _state_31
                                                                                                                            (:`NewEnumerator0`
                                                                                                                              (bind _state_32 (`self.Add Dialogue` "Sir Aeschere" "I just might be able to teach you a thing or two." (`|MakeArray` "Continue" :!type "Text") null "/Game/NPCs/friends/THEKING/HrothgarTalking_InFront.HrothgarTalking_InFront" (`self.kingAnimationSkeleton`)))
                                                                                                                              (switch `/Game/dialogueSystem/Enum_Dialogue_State` _state_32
                                                                                                                                (:`NewEnumerator0`
                                                                                                                                  (`/Game/NPCs/friends/Knight/NPC_Knight.knightWalkAway` _asnpc_knight)
                                                                                                                                  (bind (_state_33 _optionindex_2) (`self.Add Dialogue` "King Hrothgar" "I suppose now would be the time to ask questions if you hath any." (`|MakeArray` "Why is a troll killing your villagers?" "How long has Grendel been attacking you?" "What's the deal with Aeschere?" "I don't have any questions." :!type "Text") "/Game/Audio/VoiceLines/KingHrothgar/king-16.king-16" "/Game/NPCs/friends/THEKING/HrothgarTalking_InFront.HrothgarTalking_InFront" (`self.kingAnimationSkeleton`) :!label _label))
                                                                                                                                  (switch `/Game/dialogueSystem/Enum_Dialogue_State` _state_33
                                                                                                                                    (:`NewEnumerator0`
                                                                                                                                      (switch `int` _optionindex_2
                                                                                                                                        (:`0`
                                                                                                                                          (bind _state_34 (`self.Add Dialogue` "King Hrothgar" "Why? WHY? Does an evil beast need a reason to commit heinous acts? I think not!" (`|MakeArray` "Continue" :!type "Text") "/Game/Audio/VoiceLines/KingHrothgar/king-17.king-17"))
                                                                                                                                          (switch `/Game/dialogueSystem/Enum_Dialogue_State` _state_34
                                                                                                                                            (:`NewEnumerator0`
                                                                                                                                              (bind _state_35 (`self.Add Dialogue` "King Hrothgar" "He is a monster, he is vile, and I hate his stupid face!" (`|MakeArray` "Continue" :!type "Text") "/Game/Audio/VoiceLines/KingHrothgar/king-18.king-18"))
                                                                                                                                              (switch `/Game/dialogueSystem/Enum_Dialogue_State` _state_35
                                                                                                                                                (:`NewEnumerator0`
                                                                                                                                                  (bind _state_36 (`self.Add Dialogue` "King Hrothgar" "All you need to know is that he is the scum of the earth and cannot be trusted." (`|MakeArray` "Continue" :!type "Text") "/Game/Audio/VoiceLines/KingHrothgar/king-19.king-19"))
                                                                                                                                                  (switch `/Game/dialogueSystem/Enum_Dialogue_State` _state_36
                                                                                                                                                    (:`NewEnumerator0`
                                                                                                                                                      (goto _label))))))))
                                                                                                                                        (:`1`
                                                                                                                                          (bind _state_37 (`self.Add Dialogue` "King Hrothgar" "The beast has been attacking our people for months now. Every week it seems as if someone new goes missing. " (`|MakeArray` "Continue" :!type "Text") "/Game/Audio/VoiceLines/KingHrothgar/king-20.king-20"))
                                                                                                                                          (switch `/Game/dialogueSystem/Enum_Dialogue_State` _state_37
                                                                                                                                            (:`NewEnumerator0`
                                                                                                                                              (bind _state_38 (`self.Add Dialogue` "King Hrothgar" "We sent out many knights to kill him, but as you can see, he got the better of them." (`|MakeArray` "Continue" :!type "Text") "/Game/Audio/VoiceLines/KingHrothgar/king-21.king-21"))
                                                                                                                                              (switch `/Game/dialogueSystem/Enum_Dialogue_State` _state_38
                                                                                                                                                (:`NewEnumerator0`
                                                                                                                                                  (bind _state_39 (`self.Add Dialogue` "King Hrothgar" "The latest attack,  was on the village near the marsh, the biome that of Grendel's own home. " (`|MakeArray` "Continue" :!type "Text") "/Game/Audio/VoiceLines/KingHrothgar/king-22.king-22"))
                                                                                                                                                  (switch `/Game/dialogueSystem/Enum_Dialogue_State` _state_39
                                                                                                                                                    (:`NewEnumerator0`
                                                                                                                                                      (bind _state_40 (`self.Add Dialogue` "King Hrothgar" "I reccommend you ask the townsfolk there questions on the beast, maybe their information could prove valuable." (`|MakeArray` "Continue" :!type "Text") "/Game/Audio/VoiceLines/KingHrothgar/king-23.king-23"))
                                                                                                                                                      (switch `/Game/dialogueSystem/Enum_Dialogue_State` _state_40
                                                                                                                                                        (:`NewEnumerator0`
                                                                                                                                                          (goto _label))))))))))
                                                                                                                                        (:`2`
                                                                                                                                          (bind _state_41 (`self.Add Dialogue` "King Hrothgar" "Ah, fret not peasant! Aeschere is simply worried of your wellbeing. Grendel is afterall, the biggest threat the Kingdom of the Danes, it is understandable he would be upset at the thought of sending a weakli- I mean strong dirt farmer to such peril." (`|MakeArray` "Continue" :!type "Text") "/Game/Audio/VoiceLines/KingHrothgar/king-24.king-24"))
                                                                                                                                          (switch `/Game/dialogueSystem/Enum_Dialogue_State` _state_41
                                                                                                                                            (:`NewEnumerator0`
                                                                                                                                              (bind _state_42 (`self.Add Dialogue` "King Hrothgar" "Just recently, he has been diagnosed with the rare condition called ethics, which was only just discovered by our court mages. We can only hope his condition doesn't worsen." (`|MakeArray` "Continue" :!type "Text") "/Game/Audio/VoiceLines/KingHrothgar/king-25.king-25"))
                                                                                                                                              (switch `/Game/dialogueSystem/Enum_Dialogue_State` _state_42
                                                                                                                                                (:`NewEnumerator0`
                                                                                                                                                  (bind _state_43 (`self.Add Dialogue` "King Hrothgar" "Aside, he hath been by mine side for a millenia, ever since he was a young boy as a matter of fact." (`|MakeArray` "Continue" :!type "Text") "/Game/Audio/VoiceLines/KingHrothgar/king-26.king-26"))
                                                                                                                                                  (switch `/Game/dialogueSystem/Enum_Dialogue_State` _state_43
                                                                                                                                                    (:`NewEnumerator0`
                                                                                                                                                      (bind _state_44 (`self.Add Dialogue` "King Hrothgar" "You may see why he may be careful when dealing with 'new blood', as he puts it." (`|MakeArray` "Continue" :!type "Text") "/Game/Audio/VoiceLines/KingHrothgar/king-27.king-27"))
                                                                                                                                                      (switch `/Game/dialogueSystem/Enum_Dialogue_State` _state_44
                                                                                                                                                        (:`NewEnumerator0`
                                                                                                                                                          (goto _label))))))))))
                                                                                                                                        (:`3`
                                                                                                                                          (bind _state_45 (`self.Add Dialogue` "King Hrothgar" "Well, off you go now! Don't make your king wait..." (`|MakeArray` "Continue" :!type "Text") "/Game/Audio/VoiceLines/KingHrothgar/king-28.king-28"))
                                                                                                                                          (switch `/Game/dialogueSystem/Enum_Dialogue_State` _state_45
                                                                                                                                            (:`NewEnumerator0`
                                                                                                                                              (`self.setDialogueTreeIndex` 1)
                                                                                                                                              (`self.clearDialogueProgress`)
                                                                                                                                              (`self.closeConvo`)
                                                                                                                                              (`CharacterMovementComponent.SetMovementMode` (`Character.CharacterMovement` _asbp_first_person_character) "MOVE_Walking" 0)
                                                                                                                                              (set `/Game/Dynamic/FirstPerson/Blueprints/BP_FirstPersonCharacter.isIdle` false _asbp_first_person_character)
                                                                                                                                              (`/Game/NPCs/friends/Knight/NPC_Knight.moveToTrainingGrounds` _asnpc_knight)
                                                                                                                                              (bind _output_get (set `/Game/Dynamic/FirstPerson/Blueprints/levelSaveData.kingDialogueTreeIndex` 1 _as_level_save_data))
                                                                                                                                              (set `self.dialogueTreeIndex` _output_get))))))))))))))))))))))))))))))))))))))))))))))))))))))))))))))))))))))
    (:`1`
      (goto _label))))