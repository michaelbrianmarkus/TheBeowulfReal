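; Dialogue component for Sir Aeschere, the knight who tutors Beowulf through the intro.
; A switch on the saved KnightDialogueTreeIndex, overridden once Grendel is dead, runs chained AddDialogue calls that advance on Pass Through.
; Stages reveal the sword and unlock attack, then sprint and dash after the test hit, then destroy the gates and end the intro.
; The knight is found by casting the first NPC_Base actor; SaveLevelData is never reached.
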(fn `dialogue`
  (`parent.dialogue`)
  (bind _asbp_first_person_character (cast `/Game/Dynamic/FirstPerson/Blueprints/BP_FirstPersonCharacter` (`GameplayStatics.GetPlayerCharacter` 0)))
  (bind _as_level_save_data (`/Game/Dynamic/FirstPerson/Blueprints/BP_FirstPersonGameMode.As Level Save Data` (`/Game/Dynamic/FirstPerson/Blueprints/BP_FirstPersonCharacter.Game Mode` _asbp_first_person_character)))
  (set `self.dialogueTreeIndex` (`/Game/Dynamic/FirstPerson/Blueprints/levelSaveData.knightDialogueTreeIndex` _as_level_save_data))
  (bind _returnvalue (`GameplayStatics.GetActorOfClass` "/Game/dialogueSystem/NPC_Base.NPC_Base_C"))
  (bind _asnpc_knight (cast `/Game/NPCs/friends/Aeschere/NPC_Knight` _returnvalue))
  (if (`/Game/Dynamic/FirstPerson/Blueprints/levelSaveData.grendelDead?` _as_level_save_data)
    (set `self.dialogueTreeIndex` 4))
  (switch `int` (`self.dialogueTreeIndex`)
    (:`0`
      (bind _state (`self.Add Dialogue` "Sir Aeschere" "Look, I don't know what the king sees in you that I don't, but fighting Grendel in your 'current' state is a death sentence. " (`|MakeArray` "Continue" :!type "Text") null "/Game/NPCs/friends/THEKING/HrothgarTalking_InFront.HrothgarTalking_InFront"))
      (switch `/Game/dialogueSystem/Enum_Dialogue_State` _state
        (:`NewEnumerator0`
          (bind _state_2 (`self.Add Dialogue` "Sir Aeschere" "You say you can wield the blade, here take this. This sword is perfect for your size and stature. " (`|MakeArray` "Continue" :!type "Text") null "/Game/NPCs/friends/THEKING/HrothgarTalking_InFront.HrothgarTalking_InFront"))
          (switch `/Game/dialogueSystem/Enum_Dialogue_State` _state_2
            (:`NewEnumerator0`
              (`SceneComponent.SetVisibility` (`/Game/Dynamic/FirstPerson/Blueprints/BP_FirstPersonCharacter.SM_Sword` _asbp_first_person_character) true false)
              (bind (_state_3 _optionindex) (`self.Add Dialogue` "Sir Aeschere" "I want you to take that sword and hit me with it as hard as you can. " (`|MakeArray` "This is gonna hurt." "Seriously?" :!type "Text") null "/Game/NPCs/friends/THEKING/HrothgarTalking_InFront.HrothgarTalking_InFront"))
              (switch `/Game/dialogueSystem/Enum_Dialogue_State` _state_3
                (:`NewEnumerator0`
                  (switch `int` _optionindex
                    (:`0`
                      (bind _state_4 (`self.Add Dialogue` "Sir Aeschere" "Heh, well c'mon then! Hit me with your best strike! [Left Mouse Button]" (`|MakeArray` "Continue" :!type "Text") null "/Game/NPCs/friends/THEKING/HrothgarTalking_InFront.HrothgarTalking_InFront" :!label _label))
                      (switch `/Game/dialogueSystem/Enum_Dialogue_State` _state_4
                        (:`NewEnumerator0`
                          _)))
                    (:`1`
                      (bind _state_5 (`self.Add Dialogue` "Sir Aeschere" "Heh, don't worry young one! I am the strongest in all of Herot! I cannot be harmed by normal means." (`|MakeArray` "Continue" :!type "Text") null "/Game/NPCs/friends/THEKING/HrothgarTalking_InFront.HrothgarTalking_InFront"))
                      (switch `/Game/dialogueSystem/Enum_Dialogue_State` _state_5
                        (:`NewEnumerator0`
                          (bind _state_6 (`self.Add Dialogue` "Sir Aeschere" "So c'mon! Hit me with your best shot! [Left Mouse Button]" (`|MakeArray` "Continue" :!type "Text") null "/Game/NPCs/friends/THEKING/HrothgarTalking_InFront.HrothgarTalking_InFront"))
                          (switch `/Game/dialogueSystem/Enum_Dialogue_State` _state_6
                            (:`NewEnumerator0`
                              _))))))
                  (`self.clearDialogueProgress`)
                  (set `/Game/Dynamic/FirstPerson/Blueprints/BP_FirstPersonCharacter.unlockAttack?` true _asbp_first_person_character)
                  (bind _output_get (set `self.dialogueTreeIndex` 1))
                  (set `/Game/Dynamic/FirstPerson/Blueprints/levelSaveData.knightDialogueTreeIndex` _output_get _as_level_save_data)
                  (`self.closeConvo`))))))))
    (:`1`
      (if (`/Game/NPCs/friends/Aeschere/NPC_Knight.canGetHit` _asnpc_knight)
        (goto _label)
        (else
          (bind _state_7 (`self.Add Dialogue` "Sir Aeschere" "Heh, see! That was not a bad blow my friend, however raw strength alone will not take you far." (`|MakeArray` "Continue" :!type "Text") null "/Game/NPCs/friends/THEKING/HrothgarTalking_InFront.HrothgarTalking_InFront"))
          (switch `/Game/dialogueSystem/Enum_Dialogue_State` _state_7
            (:`NewEnumerator0`
              (bind _state_8 (`self.Add Dialogue` "Sir Aeschere" "Within every living being exists the potential to withstand and incarnate great feats. " (`|MakeArray` "Continue" :!type "Text") null "/Game/NPCs/friends/THEKING/HrothgarTalking_InFront.HrothgarTalking_InFront"))
              (switch `/Game/dialogueSystem/Enum_Dialogue_State` _state_8
                (:`NewEnumerator0`
                  (bind _state_9 (`self.Add Dialogue` "Sir Aeschere" "Notice just how tired you are after swinging the sword at me, as if one swing felt like a thousand." (`|MakeArray` "Continue" :!type "Text") null "/Game/NPCs/friends/THEKING/HrothgarTalking_InFront.HrothgarTalking_InFront"))
                  (switch `/Game/dialogueSystem/Enum_Dialogue_State` _state_9
                    (:`NewEnumerator0`
                      (bind _state_10 (`self.Add Dialogue` "Sir Aeschere" "It is not because you lack the endurance to do so, but rather the power. You see, the difference in power between the two of us is so great that I hardly felt your strike." (`|MakeArray` "Continue" :!type "Text") null "/Game/NPCs/friends/THEKING/HrothgarTalking_InFront.HrothgarTalking_InFront"))
                      (switch `/Game/dialogueSystem/Enum_Dialogue_State` _state_10
                        (:`NewEnumerator0`
                          (bind _state_11 (`self.Add Dialogue` "Sir Aeschere" "With power, you can do all sorts of things such as improve physical ability, cast magic, summon unworldy beings, and place illusions on the enemy. " (`|MakeArray` "Continue" :!type "Text") null "/Game/NPCs/friends/THEKING/HrothgarTalking_InFront.HrothgarTalking_InFront"))
                          (switch `/Game/dialogueSystem/Enum_Dialogue_State` _state_11
                            (:`NewEnumerator0`
                              (bind _state_12 (`self.Add Dialogue` "Sir Aeschere" "I am going to teach you one abliity that I believe will best suit your combative nature." (`|MakeArray` "Continue" :!type "Text") null "/Game/NPCs/friends/THEKING/HrothgarTalking_InFront.HrothgarTalking_InFront"))
                              (switch `/Game/dialogueSystem/Enum_Dialogue_State` _state_12
                                (:`NewEnumerator0`
                                  (bind _state_13 (`self.Add Dialogue` "Sir Aeschere" "By concentrating power to your feet you can gain the ability to run like the gods [Left Shift While Walking] and jump on the air itself [Jump While In The Air With Spacebar]. Try it out for yourself! " (`|MakeArray` "Continue" :!type "Text") null "/Game/NPCs/friends/THEKING/HrothgarTalking_InFront.HrothgarTalking_InFront"))
                                  (switch `/Game/dialogueSystem/Enum_Dialogue_State` _state_13
                                    (:`NewEnumerator0`
                                      (`self.clearDialogueProgress`)
                                      (set `/Game/Dynamic/FirstPerson/Blueprints/BP_FirstPersonCharacter.unlockSprint?` true _asbp_first_person_character)
                                      (set `/Game/Dynamic/FirstPerson/Blueprints/BP_FirstPersonCharacter.unlockDash?` true _asbp_first_person_character)
                                      (bind _output_get_2 (set `self.dialogueTreeIndex` 2))
                                      (`self.closeConvo`)
                                      (set `/Game/Dynamic/FirstPerson/Blueprints/levelSaveData.knightDialogueTreeIndex` _output_get_2 _as_level_save_data))))))))))))))))))
    (:`2`
      (bind _state_14 (`self.Add Dialogue` "Sir Aeschere" "You're quick to learn! Maybe the king was right about you..." (`|MakeArray` "Continue" :!type "Text") null "/Game/NPCs/friends/THEKING/HrothgarTalking_InFront.HrothgarTalking_InFront"))
      (switch `/Game/dialogueSystem/Enum_Dialogue_State` _state_14
        (:`NewEnumerator0`
          (bind _state_15 (`self.Add Dialogue` "Sir Aeschere" "These abilities while fine on their own, cans soar to even greater heights! You just have to know the right people. Some may be willing to help you out so long as you help them out. Increasing your reputation will get you far- erm, what is your name?" (`|MakeArray` "Continue" :!type "Text") null "/Game/NPCs/friends/THEKING/HrothgarTalking_InFront.HrothgarTalking_InFront"))
          (switch `/Game/dialogueSystem/Enum_Dialogue_State` _state_15
            (:`NewEnumerator0`
              (bind _state_16 (`self.Add Dialogue` "Beowulf" "My name is Beowulf and I WILL MURDER THAT  FOUL BEAST!" (`|MakeArray` "Continue" :!type "Text") null "/Game/NPCs/friends/THEKING/HrothgarTalking_InFront.HrothgarTalking_InFront"))
              (switch `/Game/dialogueSystem/Enum_Dialogue_State` _state_16
                (:`NewEnumerator0`
                  (bind _state_17 (`self.Add Dialogue` "Sir Aeschere" "Ah! The thrill of the hunt, how I do miss it..." (`|MakeArray` "Continue" :!type "Text") null "/Game/NPCs/friends/THEKING/HrothgarTalking_InFront.HrothgarTalking_InFront"))
                  (switch `/Game/dialogueSystem/Enum_Dialogue_State` _state_17
                    (:`NewEnumerator0`
                      (bind _state_18 (`self.Add Dialogue` "Sir Aeschere" "Beowulf, here take this. It is a map of the region so that you won't get lost on your way. Grendel's hut is located in the swamp to the east, straight ahead when you leave the city walls." (`|MakeArray` "Continue" :!type "Text") null "/Game/NPCs/friends/THEKING/HrothgarTalking_InFront.HrothgarTalking_InFront"))
                      (switch `/Game/dialogueSystem/Enum_Dialogue_State` _state_18
                        (:`NewEnumerator0`
                          (bind _state_19 (`self.Add Dialogue` "Sir Aeschere" "The gates should be open now. If you need anything, I'll be here. Otherwise, good luck Beowulf." (`|MakeArray` "Continue" :!type "Text") null "/Game/NPCs/friends/THEKING/HrothgarTalking_InFront.HrothgarTalking_InFront" :!label _label_2))
                          (switch `/Game/dialogueSystem/Enum_Dialogue_State` _state_19
                            (:`NewEnumerator0`
                              (`self.clearDialogueProgress`)
                              (bind _output_get_3 (set `self.dialogueTreeIndex` 3))
                              (set `/Game/Dynamic/FirstPerson/Blueprints/levelSaveData.knightDialogueTreeIndex` _output_get_3 _as_level_save_data)
                              (`self.closeConvo`)
                              (set `/Game/Dynamic/FirstPerson/Blueprints/levelSaveData.startIntroSequence?` false (`/Game/Dynamic/FirstPerson/Blueprints/BP_FirstPersonGameMode.As Level Save Data` (`/Game/Dynamic/FirstPerson/Blueprints/BP_FirstPersonCharacter.Game Mode` _asbp_first_person_character)))
                              (bind _outactors (`GameplayStatics.GetAllActorsOfClass` "/Game/Props/VillageProps/medieval-tower-bridge/source/destrucableGate.destrucableGate_C"))
                              (for _array_element _outactors
                                (`Actor.K2_DestroyActor` _array_element)))))))))))))))
    (:`3`
      (goto _label_2))
    (:`4`
      (bind _state_20 (`self.Add Dialogue` "Sir Aeschere" "Can't talk right now." (`|MakeArray` "Continue" :!type "Text") null "/Game/NPCs/friends/THEKING/HrothgarTalking_InFront.HrothgarTalking_InFront"))
      (switch `/Game/dialogueSystem/Enum_Dialogue_State` _state_20
        (:`NewEnumerator0`
          (`self.closeConvo`)
          (`self.clearDialogueProgress`))))))

(fn `openConvo`
  (`parent.openConvo`))