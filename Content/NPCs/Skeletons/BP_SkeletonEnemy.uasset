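; Skeleton enemy NPC that chases the Beowulf player character and deals melee damage.
; A detection overlap starts an AIMoveTo loop that repeats after each attack while the player lives, and leaving the LosePlayer volume stops active movement.
; On arrival it sets IsAttacking and enables the attack collision, whose overlap applies damage, for one of two random durations.
; Direct attack animation playback is disconnected, and StaminaDrain is an empty stub.
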(event `ChaseBeowulf`
  ;[1 0 0.6634] CHASE THE PLAYER
  (bind _asbp_first_person_character (cast `/Game/Dynamic/FirstPerson/Blueprints/BP_FirstPersonCharacter` (`GameplayStatics.GetPlayerCharacter` 0)))
  (if (not (`/Game/Dynamic/FirstPerson/Blueprints/BP_FirstPersonCharacter.isDead` _asbp_first_person_character))
    (`|AIMoveTo` self (0.0 0.0 0.0) (`GameplayStatics.GetPlayerCharacter` 0) 20.0
      (:`OnSuccess`
        (bind _output_get (set `self.Target` (`KismetMathLibrary.RandomIntegerInRange` 0 1)))
        (set `self.IsAttacking?` true)
        (`PrimitiveComponent.SetCollisionEnabled` (`self.AttackCollision`) "QueryOnly")
        (if (== _output_get 0)
          (`KismetSystemLibrary.Delay` 3.0)
          (else
            (`KismetSystemLibrary.Delay` 2.5)))
        (set `self.IsAttacking?` false)
        (`PrimitiveComponent.SetCollisionEnabled` (`self.AttackCollision`) "NoCollision")
        (`self.ChaseBeowulf`)))))

(event `self.playerDetection.OnComponentBeginOverlap`
  (params (OverlappedComponent :type "PrimitiveComponent Object Reference") (OtherActor :type "Actor Object Reference") (OtherComp :type "PrimitiveComponent Object Reference") (OtherBodyIndex :type Integer) (bFromSweep :type Boolean) (SweepResult :type "HitResult Structure (by ref)"))
  ;[1 0 0.636] Detect Player
  (cast `/Game/Dynamic/FirstPerson/Blueprints/BP_FirstPersonCharacter` OtherActor)
  (`self.ChaseBeowulf`))

(event `self.ReceiveBeginPlay`
  (`PrimitiveComponent.SetCollisionEnabled` (`self.AttackCollision`) "NoCollision"))

(event `self.losePlayer.OnComponentEndOverlap`
  (params (OverlappedComponent :type "PrimitiveComponent Object Reference") (OtherActor :type "Actor Object Reference") (OtherComp :type "PrimitiveComponent Object Reference") (OtherBodyIndex :type Integer))
  ;[1 0 0.9184] Lose sight of player
  (cast `/Game/Dynamic/FirstPerson/Blueprints/BP_FirstPersonCharacter` OtherActor)
  (`NavMovementComponent.StopActiveMovement` (`self.CharacterMovement`)))

(event `self.AttackCollision.OnComponentBeginOverlap`
  (params (OverlappedComponent :type "PrimitiveComponent Object Reference") (OtherActor :type "Actor Object Reference") (OtherComp :type "PrimitiveComponent Object Reference") (OtherBodyIndex :type Integer) (bFromSweep :type Boolean) (SweepResult :type "HitResult Structure (by ref)"))
  ;[1 0 0.5828] AttackHitPlayer
  (bind _asbp_first_person_character (cast `/Game/Dynamic/FirstPerson/Blueprints/BP_FirstPersonCharacter` OtherActor))
  (bind _asbp_first_person_character_2 (cast `/Game/Dynamic/FirstPerson/Blueprints/BP_FirstPersonCharacter` (`GameplayStatics.GetPlayerCharacter` 0)))
  (if (not (`/Game/Dynamic/FirstPerson/Blueprints/BP_FirstPersonCharacter.isDead` _asbp_first_person_character_2))
    (`GameplayStatics.ApplyDamage` _asbp_first_person_character 5.0)))

(fn `staminaDrain`)

(fn `UserConstructionScript`)