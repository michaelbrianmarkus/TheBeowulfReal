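; Dialogue component for the squire Wiglaf, who introduces himself to Beowulf and says the king requests his presence.
; It overrides Dialogue, playing a linear chain of voiced and animated AddDialogue lines at tree index 0, ending in a two-option choice.
; Exploring closes the conversation and calls ReturnToKingdom on the NPC_Wiglaf found in the level.
; Fast travel closes it and teleports the player's capsule to a hardcoded location.
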(fn `dialogue`
  (`parent.dialogue`)
  (bind _asbp_first_person_character (cast `/Game/Dynamic/FirstPerson/Blueprints/BP_FirstPersonCharacter` (`GameplayStatics.GetPlayerCharacter` 0)))
  (bind _returnvalue (`GameplayStatics.GetActorOfClass` "/Game/NPCs/friends/Wiglaf/NPC_Wiglaf.NPC_Wiglaf_C"))
  (bind _asnpc_wiglaf (cast `/Game/NPCs/friends/Wiglaf/NPC_Wiglaf` _returnvalue))
  (switch `int` (`self.dialogueTreeIndex`)
    (:`0`
      (bind _state (`self.Add Dialogue` "Wiglaf" "*pant* Whew, Beowulf sir *pant* you had no idea *pant* how hard it was to catch up with you!" (`|MakeArray` "Continue" :!type "Text") "/Game/Audio/VoiceLines/wiglaf/wiglaf-01.wiglaf-01" "/Game/NPCs/friends/THEKING/HrothgarTalking_InFront.HrothgarTalking_InFront"))
      (switch `/Game/dialogueSystem/Enum_Dialogue_State` _state
        (:`NewEnumerator0`
          (bind _state_2 (`self.Add Dialogue` "Beowulf" "Who are you?" (`|MakeArray` "Continue" :!type "Text") null "/Game/NPCs/friends/THEKING/HrothgarTalking_InFront.HrothgarTalking_InFront"))
          (switch `/Game/dialogueSystem/Enum_Dialogue_State` _state_2
            (:`NewEnumerator0`
              (bind _state_3 (`self.Add Dialogue` "Wiglaf" " I-I am your newly appointed s-squire. P-Pleased to meet you Beowulf-er SIR! Name’s Wiglaf!" (`|MakeArray` "Continue" :!type "Text") "/Game/Audio/VoiceLines/wiglaf/wiglaf-02.wiglaf-02" "/Game/NPCs/friends/THEKING/HrothgarTalking_InFront.HrothgarTalking_InFront"))
              (switch `/Game/dialogueSystem/Enum_Dialogue_State` _state_3
                (:`NewEnumerator0`
                  (bind _state_4 (`self.Add Dialogue` "Wiglaf" "God I hope I made a good first impression." (`|MakeArray` "Continue" :!type "Text") "/Game/Audio/VoiceLines/wiglaf/wiglaf-03.wiglaf-03" "/Game/NPCs/friends/THEKING/HrothgarTalking_InFront.HrothgarTalking_InFront"))
                  (switch `/Game/dialogueSystem/Enum_Dialogue_State` _state_4
                    (:`NewEnumerator0`
                      (bind _state_5 (`self.Add Dialogue` "Beowulf" "Y’know I can still hear you, right?" (`|MakeArray` "Continue" :!type "Text") null "/Game/NPCs/friends/THEKING/HrothgarTalking_InFront.HrothgarTalking_InFront"))
                      (switch `/Game/dialogueSystem/Enum_Dialogue_State` _state_5
                        (:`NewEnumerator0`
                          (bind _state_6 (`self.Add Dialogue` "Wiglaf" "AH JEEZ! I uh d-didn’t say anything! It was probably the wind! A-Anyways, I came by to tell you that the king requests your p-presence!" (`|MakeArray` "Continue" :!type "Text") "/Game/Audio/VoiceLines/wiglaf/wiglaf-04.wiglaf-04" "/Game/NPCs/friends/THEKING/HrothgarTalking_InFront.HrothgarTalking_InFront"))
                          (switch `/Game/dialogueSystem/Enum_Dialogue_State` _state_6
                            (:`NewEnumerator0`
                              (bind (_state_7 _optionindex) (`self.Add Dialogue` "Wiglaf" "I can take you there if you want, so you don’t have to make the journey!" (`|MakeArray` "Nope I wanna enjoy the scenery (Explore)" "Exercise? More like extra fries!  \n(Fast Travel)" :!type "Text") "/Game/Audio/VoiceLines/wiglaf/wiglaf-05.wiglaf-05" "/Game/NPCs/friends/THEKING/HrothgarTalking_InFront.HrothgarTalking_InFront"))
                              (switch `/Game/dialogueSystem/Enum_Dialogue_State` _state_7
                                (:`NewEnumerator0`
                                  (switch `int` _optionindex
                                    (:`0`
                                      (`self.closeConvo`)
                                      (`/Game/NPCs/friends/Wiglaf/NPC_Wiglaf.return to kingdom` _asnpc_wiglaf))
                                    (:`1`
                                      (`self.closeConvo`)
                                      (`SceneComponent.K2_SetWorldLocation` (`Character.CapsuleComponent` _asbp_first_person_character) (124645.184691 74749.696198 2109.478168) false true))))))))))))))))))))